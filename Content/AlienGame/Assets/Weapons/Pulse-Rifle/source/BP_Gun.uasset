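; BP_Gun is a weapon actor for the pulse rifle that fires bullets at a limited rate.
; Attack spawns a BP_Bullet at the Arrow component and calls MoveTo to send it Range units along the arrow's forward vector over a fixed time.
; A DoOnce gate blocks further shots until a Rate delay ends and UnlockAttack resets it.
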(event `self.ReceiveTick`
  (params (DeltaSeconds :type "Float (single-precision)"))
  (`parent.ReceiveTick` DeltaSeconds))

(event `/Game/AlienGame/Assets/Weapons/Pulse-Rifle/source/BPI_Weapon.Attack`
  (bind _arrow (`self.Arrow`))
  (bind _arrow_2 (`self.Arrow`))
  (`/Engine/EditorBlueprintResources/StandardMacros.DoOnce` false :!label _label
    (:`Completed`
      (`|ExecutionSequence`
        (:`then_0`
          (bind _returnvalue (`|SpawnActorFromClass` "/Game/AlienGame/Assets/Weapons/Pulse-Rifle/source/BP_Bullet.BP_Bullet_C" (`KismetMathLibrary.MakeTransform` (`SceneComponent.K2_GetComponentLocation` _arrow_2) (`SceneComponent.K2_GetComponentRotation` _arrow_2)) "Undefined" "OverrideRootScale" null null))
          (`/Game/AlienGame/Assets/Weapons/Pulse-Rifle/source/BP_Bullet.Move To` _returnvalue (+ (`SceneComponent.K2_GetComponentLocation` _arrow) (* (`SceneComponent.GetForwardVector` _arrow) (`self.Range`))) 0.35))
        (:`then_1`
          (`KismetSystemLibrary.Delay` (`self.Rate`))
          (`self.UnlockAttack`))))))

(event `UnlockAttack`
  (goto _label :!via `Reset`))

(fn `UserConstructionScript`
  (`parent.UserConstructionScript`))